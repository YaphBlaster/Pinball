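; Pinball game mode that keeps a ball in play and tracks the score.
; On BeginPlay it spawns a BP_Ball at the spawn location supplied by the first BP_Plunger found in the level.
; It binds to each ball's OnDestroyed event to spawn a replacement, with no limit on the number of balls.
; AddScore scales incoming points by the Multiplier, adds them to Score and returns the new total.
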(event Custom|SpawnBall
  (bind _outactors (Actor|GetAllActorsOfClass "/Game/Blueprints/BP_Plunger.BP_Plunger_C"))
  (bind _returnvalue (Game|SpawnActorfromClass "/Game/Blueprints/BP_Ball.BP_Ball_C" (Math|Transform|MakeTransform (Default|GetBallSpawnLocation (Utilities|Array|Get(acopy) _outactors)) "0, 0, 0" "1,1,1") "Undefined" 0 0))
  (Game|BindEventtoOnDestroyed _returnvalue (delegate Custom|OnBallDestroyed)))

(event Custom|OnBallDestroyed
  (params (DestroyedActor :type Actor%20Object%20Reference))
  (CallFunction|SpawnBall))

(event EventBeginPlay
  (CallFunction|SpawnBall))

(event EventTick
  (params (DeltaSeconds :type Float%20%28single-precision%29)))

(fn ConstructionScript)

(fn AddScore
  (params (PointsToAdd :type Float%20%28single-precision%29))
  (bind _output_get (Variables|Default|SetScore (+ (* PointsToAdd (Variables|Default|GetMultiplier)) (Variables|Default|GetScore))))
  (return _output_get))